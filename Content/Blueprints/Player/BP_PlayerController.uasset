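; Player controller that opens the pause menu from keyboard or gamepad input.
; It creates a W_MainWidget on BeginPlay, then the IA_menu and IA_GamepadMenu actions add it to the viewport, switch to UI-only input and pause the game.
; The IA_menu path also sets keyboard focus and shows the mouse cursor, while the gamepad path hides the cursor.
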(event Input|EnhancedActionEvents|EnhancedInputActionIA_menu
  (params (ActionValue :type Boolean) (ElapsedSeconds :type Float%20%28double-precision%29) (TriggeredSeconds :type Float%20%28double-precision%29) (InputAction :type Input%20Action%20Object%20Reference :default "/Game/Blueprints/Input/IA_menu.IA_menu"))
  (bind _returnvalue (Game|GetPlayerController 0))
  (bind _widget (Variables|Default|GetWidget))
  ;[1 1 1] Выход в меню
  (:Started
    (UserInterface|Viewport|AddtoViewport _widget 0)
    (Widget|SetKeyboardFocus _widget)
    (Input|SetInputModeUIOnly _returnvalue _widget "DoNotLock" false)
    (Variables|/Script/Engine.PlayerController|SetbShowMouseCursor _returnvalue true)
    (Game|SetGamePaused true)))

(event Input|EnhancedActionEvents|EnhancedInputActionIA_GamepadMenu
  (params (ActionValue :type Boolean) (ElapsedSeconds :type Float%20%28double-precision%29) (TriggeredSeconds :type Float%20%28double-precision%29) (InputAction :type Input%20Action%20Object%20Reference :default "/Game/Blueprints/Input/IA_GamepadMenu.IA_GamepadMenu"))
  (bind _returnvalue (Game|GetPlayerController 0))
  (bind _widget (Variables|Default|GetWidget))
  ;[1 1 1] Выход в меню геймпад
  (:Started
    (UserInterface|Viewport|AddtoViewport _widget 0)
    (Input|SetInputModeUIOnly _returnvalue _widget "DoNotLock" false)
    (Variables|/Script/Engine.PlayerController|SetbShowMouseCursor _returnvalue false)
    (Game|SetGamePaused true)))

(event EventBeginPlay
  ;[1 1 1] Create widget
  (bind _returnvalue (UserInterface|CreateWidget "/Game/Blueprints/UI/W_MainWidget.W_MainWidget_C" (Game|GetPlayerController 0)))
  (Variables|Default|SetWidget _returnvalue))

(event EventTick
  (params (DeltaSeconds :type Float%20%28single-precision%29)))

(fn ConstructionScript)